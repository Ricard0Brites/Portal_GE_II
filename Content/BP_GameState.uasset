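; Game state Blueprint that hands out mesh colors to player characters in rotating order.
; SR_RequestColor sets the requesting character's MeshColor from the Color array at a running player counter, then increments it.
; A bounds check before each assignment wraps the counter to zero, so colors repeat once the array runs out.
; The counter resets on BeginPlay, and the Clients Color OnRep handler is empty.
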(event `self.ReceiveBeginPlay`
  (set `self.Player Running Count` 0))

(event `SR_RequestColor`
  (params (`As Player Character` :type "/Game/FirstPersonCharacter Object Reference"))
  (if (not (<= (`self.Player Running Count`) (- (`KismetArrayLibrary.Array_Length` (`self.Color`)) 1)))
    (set `self.Player Running Count` 0))
  (set `/Game/FirstPersonCharacter.MeshColor` (`|GetArrayItem` (`self.Color`) (`self.Player Running Count`)) `As Player Character`)
  (`self.Increment Client Counter`))

(fn `OnRep_Clients Color`)

(fn `UserConstructionScript`)