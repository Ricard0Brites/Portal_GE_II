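; Weapon platform Blueprint that displays a colored hologram mesh, with events to enable or disable it.
; ChangeGunMeshColor, noted as triggered from C++ on BeginPlay, sets the replicated WeaponColor.
; Its OnRep creates a dynamic M_Hologram material instance with that color and applies it to the mesh.
; Enable and disable events toggle the hologram's visibility and the box collider between query-only and no collision.
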(event `self.ChangeGunMeshColor`
  (params (ColorToChangeTo :type "LinearColor Structure"))
  ;[1 1 1] Replicated Color Change
  ; Triggered on BeginPlay (C++)
  (set `self.WeaponColor` ColorToChangeTo))

(event `self.DisableHologramComponent`
  (`PrimitiveComponent.SetCollisionEnabled` (`self.boxCollider`) "NoCollision")
  (`SceneComponent.SetVisibility` (`self.hologramMesh`) false false))

(event `self.EnableHologramComponent`
  (`PrimitiveComponent.SetCollisionEnabled` (`self.boxCollider`) "QueryOnly")
  (`SceneComponent.SetVisibility` (`self.hologramMesh`) true false))

(fn `OnRep_WeaponColor`
  (bind _hologrammesh (`self.hologramMesh`))
  (bind _returnvalue (`PrimitiveComponent.CreateDynamicMaterialInstance` _hologrammesh 0 "/Game/FPWeapon/Materials/M_Hologram.M_Hologram" "None"))
  (`MaterialInstanceDynamic.SetVectorParameterValue` _returnvalue "Color" (`self.WeaponColor`))
  (`PrimitiveComponent.SetMaterial` _hologrammesh 0 _returnvalue))

(fn `UserConstructionScript`)